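; BP_Character is a player character with mouse-look style camera input, sprinting, and yaw that eases toward control rotation while moving.
; Move axes only store InputForward and InputRight, doubled during sprint, with BlockInput gating just the right axis; Sprint also switches max walk speed.
; The Jump action fires a debug-drawn object trace from the camera, while actual jumping and BP_Ball spawning logic sit unconnected.
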(event EventTick
  (params (DeltaSeconds :type Float%20%28single-precision%29))
  (if (> (Math|Vector|VectorLength (Transformation|GetVelocity)) 1e+01)
    (Transformation|SetActorRotation (Math|Rotator|MakeRotator 0.0 0.0 (.yaw (Math|Interpolation|RInterpTo (Transformation|GetActorRotation) (Pawn|GetControlRotation :!class /Script/Engine.Pawn) DeltaSeconds 2.0))))))

(event Input|ActionEvents|InputActionJump
  (params (Key :type Key%20Structure :default "None"))
  (bind _returnvalue (Game|GetPlayerCameraManager 0))
  (bind _returnvalue_2 (Transformation|GetActorLocation _returnvalue))
  (:Pressed
    (Collision|LineTraceForObjects _returnvalue_2 (+ _returnvalue_2 (* (Transformation|GetActorForwardVector _returnvalue) 1e+03)) (Utilities|Array|MakeArray "ObjectTypeQuery1" "ObjectTypeQuery2") false 0 "ForDuration")))

(event Input|ActionEvents|InputActionSprint
  (params (Key :type Key%20Structure :default "None"))
  (:Pressed
    (Variables|Default|SetIsSprint true)
    (Variables|/Script/Engine.CharacterMovementComponent|SetMaxWalkSpeed (Variables|Character|GetCharacterMovement) 6e+02))
  (:Released
    (Variables|Default|SetIsSprint false)
    (Variables|/Script/Engine.CharacterMovementComponent|SetMaxWalkSpeed (Variables|Character|GetCharacterMovement) 1.8e+02)))

(event Input|AxisEvents|InputAxisMoveForward
  (params (AxisValue :type Float%20%28single-precision%29))
  (Variables|Default|SetInput%20Forward (select (Variables|Default|GetIsSprint) (* AxisValue 2.0) AxisValue)))

(event Input|AxisEvents|InputAxisMoveright
  (params (AxisValue :type Float%20%28single-precision%29))
  (if (not (Variables|Default|GetBlockInput))
    (Variables|Default|SetInput%20Right (select (Variables|Default|GetIsSprint) (* AxisValue 2.0) AxisValue))))

(event Input|AxisEvents|InputAxisLookUp
  (params (AxisValue :type Float%20%28single-precision%29))
  (Pawn|Input|AddControllerPitchInput AxisValue))

(event Input|AxisEvents|InputAxisLookRight
  (params (AxisValue :type Float%20%28single-precision%29))
  (Pawn|Input|AddControllerYawInput AxisValue))

(fn ConstructionScript)